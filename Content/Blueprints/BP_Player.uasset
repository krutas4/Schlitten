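; BP_Player is the player character, which constantly moves forward on its own in a sliding ("Rutschen") mechanic, with mouse look and jump.
; Each Tick, Rutschen compares the heights of the Hinten (back) and Vorne (front) components, adding a Speed-based offset to forward input when the back is lower.
; BeginPlay registers the Enhanced Input mapping context.
; Slope-angle and floor-alignment experiments remain as unconnected nodes.
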(event Custom|CustomEvent
  (bind _charactermovement (Variables|Character|GetCharacterMovement))
  (if (not (AI|Components|NavMovement|IsFalling _charactermovement))
    (bind _output_get (Variables|Default|SetSlideAngle (Class|KismetMathLibrary|DegAcos (Math|Vector|DotProduct (.ImpactNormal (Collision|BreakHitResult (.HitResult (Utilities|Struct|BreakFindFloorResult (Variables|/Script/Engine.CharacterMovementComponent|GetCurrentFloor _charactermovement))))) "0.000000,0.000000,1.000000"))))
    (if (< _output_get 3e+01)
      _)))

(event Custom|CustomEvent_1)

(event Collision|EventActorBeginOverlap
  (params (OtherActor :type Actor%20Object%20Reference)))

(event EventBeginPlay
  (CallFunction|Inputs))

(event EventTick
  (params (DeltaSeconds :type Float%20%28single-precision%29))
  (CallFunction|Rutschen))

(event Custom|Inputs
  (Input|AddMappingContext (PlayerController|LocalPlayerSubsystems|GetEnhancedInputLocalPlayerSubsystem (Game|GetPlayerController 0)) "/Game/Inputs/IMC_Player.IMC_Player" 0 "(bIgnoreAllPressedKeysUntilRelease=True,bForceImmediately=False)"))

(event Custom|Rutschen
  (if (< (.z (Transformation|GetWorldLocation (Variables|Default|GetHinten))) (.z (Transformation|GetWorldLocation (Variables|Default|GetVorne))))
    (Pawn|Input|AddMovementInput (+ (Transformation|GetActorForwardVector) (* (Variables|Default|GetSpeed) (Utilities|Time|GetWorldDeltaSeconds))) 1.0 false)
    (else
      (Pawn|Input|AddMovementInput (+ (Transformation|GetActorForwardVector) (* 1.0 (Utilities|Time|GetWorldDeltaSeconds))) 1.0 false))))

(event Input|EnhancedActionEvents|EnhancedInputActionIA_Movement
  (params (ActionValue :type Vector%202D%20Structure) (ElapsedSeconds :type Float%20%28double-precision%29) (TriggeredSeconds :type Float%20%28double-precision%29) (InputAction :type Input%20Action%20Object%20Reference :default "/Game/Inputs/IA_Movement.IA_Movement")))

(event Input|EnhancedActionEvents|EnhancedInputActionIA_Look
  (params (ActionValue :type Vector%202D%20Structure) (ElapsedSeconds :type Float%20%28double-precision%29) (TriggeredSeconds :type Float%20%28double-precision%29) (InputAction :type Input%20Action%20Object%20Reference :default "/Game/Inputs/IA_Look.IA_Look"))
  (bind _mousesensitivity (Variables|Default|GetMouseSensitivity))
  (:Triggered
    (Pawn|Input|AddControllerYawInput (* _mousesensitivity (.x ActionValue)))
    (Pawn|Input|AddControllerPitchInput (* (* (.y ActionValue) _mousesensitivity) -1.0))))

(event Input|EnhancedActionEvents|EnhancedInputActionIA_Jump
  (params (ActionValue :type Boolean) (ElapsedSeconds :type Float%20%28double-precision%29) (TriggeredSeconds :type Float%20%28double-precision%29) (InputAction :type Input%20Action%20Object%20Reference :default "/Game/Inputs/IA_Jump.IA_Jump"))
  (:Started
    (Character|Jump)))

(fn ConstructionScript)