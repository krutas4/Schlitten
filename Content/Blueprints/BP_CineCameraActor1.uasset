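; BP_CineCameraActor1 is a camera that follows the player along a camera spline while turning to look at them.
; Each tick it rotates the camera toward PlayerPawn and finds the point on CameraSplineRef's spline nearest the player pawn.
; A helper event converts that point to a spline distance by interpolating between neighboring points, and the camera eases there with VInterpTo.
; BeginPlay stores a found BP_CameraSpline in SplinePoints, whereas Tick reads CameraSplineRef.
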(event Custom|Find%20Distance%20Along%20Spline%20Closest%20to%20World%20Location
  (params (Location :type Vector) (Spline :type Spline%20Component%20Object%20Reference))
  (bind _returnvalue (Class|SplineComponent|FindInputKeyClosesttoWorldLocation Spline Location))
  (bind _returnvalue_2 (Math|Float|Truncate _returnvalue))
  (bind _returnvalue_3 (Spline|GetDistanceAlongSplineatSplinePoint Spline _returnvalue_2))
  (Variables|Default|SetActualSplineDistance (+ _returnvalue_3 (* (- (Spline|GetDistanceAlongSplineatSplinePoint Spline (Math|Float|Truncate (+ _returnvalue 1.0))) _returnvalue_3) (- _returnvalue (Math|Conversions|ToFloat(Integer) _returnvalue_2))))))

(event EventBeginPlay
  (bind _returnvalue (Actor|GetActorOfClass "/Game/Blueprints/BP_CameraSpline.BP_CameraSpline_C"))
  (Variables|Default|SetSplinePoints _returnvalue))

(event EventTick
  (params (DeltaSeconds :type Float%20%28single-precision%29))
  (bind _cameracomponent (Variables|CameraActor|GetCameraComponent))
  (bind _playerpawn (Variables|Default|GetPlayerPawn))
  (bind _camerasplineref (Variables|Default|GetCameraSplineRef))
  (bind _returnvalue (Transformation|GetWorldLocation _cameracomponent))
  (bind _rootcomponent (Variables|/Script/Engine.Actor|GetRootComponent _playerpawn))
  (bind _spline (Variables|/Game/Blueprints/BP_CameraSpline.BP_CameraSpline_C|GetSpline _camerasplineref))
  (bind _returnvalue_2 (Transformation|GetWorldLocation _rootcomponent))
  (bind _returnvalue_3 (Math|Rotator|FindLookatRotation _returnvalue _returnvalue_2))
  (Transformation|SetWorldRotation (Variables|CameraActor|GetCameraComponent) (Math|Rotator|MakeRotator (.roll _returnvalue_3) (.pitch _returnvalue_3) (.yaw _returnvalue_3)) false false)
  (CallFunction|FindDistanceAlongSplineClosesttoWorldLocation (Spline|FindLocationClosesttoWorldLocation _spline (Transformation|GetActorLocation (Game|Player|GetPlayerPawn 0)) "World") _spline)
  (Transformation|SetWorldLocation (Variables|CameraActor|GetCameraComponent) (Math|Interpolation|VInterpTo (Transformation|GetWorldLocation (Variables|CameraActor|GetCameraComponent)) (Spline|GetLocationatDistanceAlongSpline (Variables|/Game/Blueprints/BP_CameraSpline.BP_CameraSpline_C|GetSpline (Variables|Default|GetCameraSplineRef)) (Variables|Default|GetActualSplineDistance) "World") (Utilities|Time|GetWorldDeltaSeconds) 0.5) false false))

(fn ConstructionScript)