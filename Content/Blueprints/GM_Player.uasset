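; GM_Player is the game mode that hands the player pawn to the first controller and manages pausing.
; BeginPlay finds the placed Pawn_Player, calls its Possesed event, creates WBP_GameUI and hides the cursor.
; PauseGame toggles pause, pushing a pause menu onto the UI's widget stack and viewport or clearing the stack.
; It also switches input mode and cursor visibility to match.
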(event Custom|PauseGame
  (bind _returnvalue (Game|GetPlayerController 0))
  (bind _gameui (Variables|Default|GetGameUI))
  (bind _pausemenustack (Variables|/Game/Blueprints/UI/WBP_GameUI.WBP_GameUI_C|GetPauseMenuStack _gameui))
  (if (not (Game|IsGamePaused))
    (bind _returnvalue_2 (Class|CommonActivatableWidgetContainerBase|AddWidget _pausemenustack "/Game/Blueprints/UI/WBP_PauseMenuBase.WBP_PauseMenuBase_C"))
    (UserInterface|Viewport|AddtoViewport _returnvalue_2 0)
    (Game|SetGamePaused true)
    (Input|SetInputModeUIOnly _returnvalue 0 "DoNotLock" false)
    (Variables|/Script/Engine.PlayerController|SetbShowMouseCursor _returnvalue true)
    (else
      (Class|CommonActivatableWidgetContainerBase|ClearWidgets _pausemenustack)
      (Game|SetGamePaused false)
      (Input|SetInputModeGameOnly _returnvalue false)
      (Variables|/Script/Engine.PlayerController|SetbShowMouseCursor _returnvalue false))))

(event EventBeginPlay
  (bind _returnvalue (Actor|GetActorOfClass "/Game/Blueprints/Pawn_Player.Pawn_Player_C"))
  (Default|Possesed _returnvalue (Game|GetPlayerController 0))
  (bind _returnvalue_2 (UserInterface|CreateWidget "/Game/Blueprints/UI/WBP_GameUI.WBP_GameUI_C"))
  (Variables|Default|SetGameUI _returnvalue_2)
  (Variables|/Script/Engine.PlayerController|SetbShowMouseCursor (Game|GetPlayerController 0) false))

(event EventTick
  (params (DeltaSeconds :type Float%20%28single-precision%29)))

(fn ConstructionScript)