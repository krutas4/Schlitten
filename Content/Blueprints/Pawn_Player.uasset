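; Player pawn that moves as a physics-driven Box under constant forward thrust and downforce along its local up axis, applied every tick.
; On possession it adds IMC_Player for Enhanced Input.
; Movement input applies a signed force and yaw to the Box, with a Timeline ramping the turn rate while held.
; Forward input applies a one-shot forward or backward turbo force on press, and look input rotates the Camera.
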(event Custom|SetupInput
  (params (Input :type Player%20Controller%20Object%20Reference))
  (Input|AddMappingContext (PlayerController|LocalPlayerSubsystems|GetEnhancedInputLocalPlayerSubsystem Input) "/Game/Inputs/IMC_Player.IMC_Player" 0 "(bIgnoreAllPressedKeysUntilRelease=True,bForceImmediately=False)"))

(event Custom|Possesed
  (params (PlayerController :type Player%20Controller%20Object%20Reference))
  (Pawn|Possess PlayerController self))

(event Custom|DownForce
  (Physics|AddForce (Variables|Default|GetBox) (* (* (Transformation|GetActorUpVector) (Variables|Default|Getgravity)) -1.0) "None" false))

(event Input|EnhancedActionEvents|EnhancedInputActionIA_Look
  (params (ActionValue :type Vector%202D%20Structure) (ElapsedSeconds :type Float%20%28double-precision%29) (TriggeredSeconds :type Float%20%28double-precision%29) (InputAction :type Input%20Action%20Object%20Reference :default "/Game/Inputs/IA_Look.IA_Look"))
  (bind _mousesensitivity (Variables|Default|GetMouseSensitivity))
  (:Triggered
    (Transformation|AddRelativeRotation (Variables|Default|GetCamera) (Math|Rotator|MakeRotator 0.0 (* (* (.y ActionValue) _mousesensitivity) -1.0) (* _mousesensitivity (.x ActionValue))) false false)))

(event Input|EnhancedActionEvents|EnhancedInputActionIA_Jump
  (params (ActionValue :type Boolean) (ElapsedSeconds :type Float%20%28double-precision%29) (TriggeredSeconds :type Float%20%28double-precision%29) (InputAction :type Input%20Action%20Object%20Reference :default "/Game/Inputs/IA_Jump.IA_Jump")))

(event Input|EnhancedActionEvents|EnhancedInputActionIA_Movement
  (params (ActionValue :type Vector%202D%20Structure) (ElapsedSeconds :type Float%20%28double-precision%29) (TriggeredSeconds :type Float%20%28double-precision%29) (InputAction :type Input%20Action%20Object%20Reference :default "/Game/Inputs/IA_Movement.IA_Movement"))
  (bind _box (Variables|Default|GetBox))
  (bind _box_2 (Variables|Default|GetBox))
  (bind _movement (Variables|Default|GetMovement))
  (:Triggered
    (switch int (Math|Float|Truncate (Math|Float|Clamp(Float) (.x ActionValue)))
      (:0
        (Physics|AddForce _box_2 (Math|Conversions|ToVector(Float) (* _movement 1.0)) "None" false)
        (Transformation|AddRelativeRotation _box (Math|Rotator|MakeRotator 0.0 0.0 (* (Math|Float|Lerp 0.1 4.0 (stale _newtrack_0)) -1.0)) false false))
      (:1
        (Physics|AddForce _box_2 (Math|Conversions|ToVector(Float) (* _movement -1.0)) "None" false)
        (Transformation|AddRelativeRotation _box (Math|Rotator|MakeRotator 0.0 0.0 (Math|Float|Lerp 0.1 4.0 (stale _newtrack_0))) false false))))
  (:Started
    (bind _newtrack_0 (Timeline|Timeline PlayFromStart)))
  (:Canceled
    (Timeline|Timeline Stop))
  (:Completed
    (Timeline|Timeline Stop)))

(event Input|EnhancedActionEvents|EnhancedInputActionIA_Forward
  (params (ActionValue :type Float%20%28double-precision%29) (ElapsedSeconds :type Float%20%28double-precision%29) (TriggeredSeconds :type Float%20%28double-precision%29) (InputAction :type Input%20Action%20Object%20Reference :default "/Game/Inputs/IA_Forward.IA_Forward"))
  (:Started
    (if (> ActionValue 0.1)
      (Physics|AddForce (Variables|Default|GetBox) (* (Transformation|GetActorForwardVector) (Variables|Default|GetTurbo)) "None" false)
      (else
        (Physics|AddForce (Variables|Default|GetBox) (* (* (Transformation|GetActorForwardVector) (Variables|Default|GetTurbo)) -1.0) "None" false)))))

(event EventBeginPlay)

(event Collision|EventActorBeginOverlap
  (params (OtherActor :type Actor%20Object%20Reference)))

(event EventTick
  (params (DeltaSeconds :type Float%20%28single-precision%29))
  (CallFunction|DownForce)
  (Physics|AddForce (Variables|Default|GetBox) (* (Transformation|GetActorForwardVector) (Variables|Default|GetSpeed)) "None" false))

(event EventPossessed
  (params (NewController :type Controller%20Object%20Reference))
  (bind _asplayer_controller (Utilities|Casting|CastToPlayerController NewController))
  (CallFunction|SetupInput self _asplayer_controller))

(fn ConstructionScript)